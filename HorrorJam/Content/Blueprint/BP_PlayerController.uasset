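; Player controller that owns the pause menu and toggles it with the Escape key.
; On BeginPlay it creates the BP_Pause widget and adds it to the viewport for the whole session.
; Escape checks the visibility of the widget's PauseBorder, then shows or hides it while setting game pause and mouse cursor to match.
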(event `self.ReceiveBeginPlay`
  (`parent.ReceiveBeginPlay`)
  (bind _returnvalue (`|CreateWidget` "/Game/Blueprint/Widgets/BP_Pause.BP_Pause_C" self))
  (bind _output_get (set `self.PauseMenu` _returnvalue))
  (`UserWidget.AddToViewport` _output_get 0))

(event `Key|Escape`
  (params (Key :type "Key Structure"))
  (bind _pauseborder (`/Game/Blueprint/Widgets/BP_Pause.PauseBorder` (`self.PauseMenu`)))
  (:`Pressed`
    (if (`Widget.IsVisible` (`/Game/Blueprint/Widgets/BP_Pause.PauseBorder` (`self.PauseMenu`)))
      (set `Widget.Visibility` "Hidden" _pauseborder)
      (`GameplayStatics.SetGamePaused` false)
      (set `self.bShowMouseCursor` false)
      (else
        (set `Widget.Visibility` "Visible" _pauseborder)
        (`GameplayStatics.SetGamePaused` true)
        (set `self.bShowMouseCursor` true)))))

(fn `UserConstructionScript`
  (`parent.UserConstructionScript`))